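; Capture point Blueprint that plays a team-colored confetti effect when it is captured.
; On capture, it spawns the confetti emitter at four scene component locations.
; It then gets the owning team's color from BaseGameMode and applies it to the Color parameter of all four emitters.
; BeginPlay, overlap, Tick and the construction script hold no logic.
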(event `self.OnCapture`
  (bind _returnvalue (`GameplayStatics.SpawnEmitterAtLocation` "/Game/Confetti_new.Confetti_new" (`SceneComponent.K2_GetComponentLocation` (`self.Scene`))))
  (bind _returnvalue_2 (`GameplayStatics.SpawnEmitterAtLocation` "/Game/Confetti_new.Confetti_new" (`SceneComponent.K2_GetComponentLocation` (`self.Scene1`))))
  (bind _returnvalue_3 (`GameplayStatics.SpawnEmitterAtLocation` "/Game/Confetti_new.Confetti_new" (`SceneComponent.K2_GetComponentLocation` (`self.Scene2`))))
  (bind _returnvalue_4 (`GameplayStatics.SpawnEmitterAtLocation` "/Game/Confetti_new.Confetti_new" (`SceneComponent.K2_GetComponentLocation` (`self.Scene3`))))
  (bind _asbase_game_mode (cast `BaseGameMode` (`GameplayStatics.GetGameMode`)))
  (`ParticleSystemComponent.SetColorParameter` _returnvalue_4 "Color" (`BaseGameMode.GetTeamColor` _asbase_game_mode (`self.m_OwningTeam`)))
  (`ParticleSystemComponent.SetColorParameter` _returnvalue_3 "Color" (`BaseGameMode.GetTeamColor` _asbase_game_mode (`self.m_OwningTeam`)))
  (`ParticleSystemComponent.SetColorParameter` _returnvalue_2 "Color" (`BaseGameMode.GetTeamColor` _asbase_game_mode (`self.m_OwningTeam`)))
  (`ParticleSystemComponent.SetColorParameter` _returnvalue "Color" (`BaseGameMode.GetTeamColor` _asbase_game_mode (`self.m_OwningTeam`))))

(fn `UserConstructionScript`)