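; Blueprint that drives in-game music through Wwise from the start of play.
; BeginPlay posts the music event, steps up a volume RTPC, and runs parallel timed delays that switch music states between levels and finally Victory, also setting a Stormtime flag late on.
; Tick maps the game mode's timer-to-duration ratio onto an interpolated Intensity RTPC.
; UI sound and storm/thunder calls exist but are unconnected.
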(event `self.ReceiveBeginPlay`
  (`AkGameplayStatics.SetState` "Music" "Level_1")
  (`AkGameplayStatics.PostEvent` "/Game/Audio/Events/Music/Music_Start.Music_Start")
  (`|ExecutionSequence`
    (:`then_0`
      (`AkGameplayStatics.SetRTPCValue` "Vol_Start")
      (`KismetSystemLibrary.Delay` 0.7)
      (`AkGameplayStatics.SetRTPCValue` "Vol_Start" 100.0))
    (:`then_1`
      (`KismetSystemLibrary.Delay` 60.0)
      (`AkGameplayStatics.SetState` "Music" "Level_1" :!label _label))
    (:`then_2`
      (`KismetSystemLibrary.Delay` 190.0)
      (`AkGameplayStatics.SetState` "Music" "Level_3"))
    (:`then_3`
      (`KismetSystemLibrary.Delay` 230.0)
      (`AkGameplayStatics.SetState` "Music" "Level_4"))
    (:`then_4`
      (`KismetSystemLibrary.Delay` 299.0)
      (`AkGameplayStatics.SetState` "Music" "Victory"))
    (:`then_5`
      (`KismetSystemLibrary.Delay` 30.0)
      (`AkGameplayStatics.SetState` "Music" "Level_2" :!label _label_2))
    (:`then_6`
      (`KismetSystemLibrary.Delay` 120.0)
      (goto _label))
    (:`then_7`
      (`KismetSystemLibrary.Delay` 90.0)
      (goto _label_2))
    (:`then_8`
      (`KismetSystemLibrary.Delay` 160.0)
      (goto _label_2))
    (:`then_9`
      (`KismetSystemLibrary.Delay` 250.0)
      (set `self.Stormtime` true))))

(event `self.ReceiveTick`
  (params (DeltaSeconds :type "Float (single-precision)"))
  (bind _asbase_game_mode (cast `BaseGameMode` (`GameplayStatics.GetGameMode`)))
  (`AkGameplayStatics.SetRTPCValue` "Intensity" (* (/ (`BaseGameMode.m_Timer` _asbase_game_mode) (`BaseGameMode.m_GameDuration` _asbase_game_mode)) 100.0) 200))

(fn `UserConstructionScript`)