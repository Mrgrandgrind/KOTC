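; Game mode for a local multiplayer team flag match, handling player setup, spawn placement and end conditions.
; On BeginPlay it creates players, assigns teams and slots by player count and PVP mode, then moves characters to matching spawn points after a delay.
; A one-second timer loop calls GameOver at the time limit or when a build area overlaps another team's flag block, recording that area's team as winner.
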(event `Game Over`)

(event `Counter`
  (bind _time (`self.Time`))
  (`KismetSystemLibrary.Delay` 1.0 :!label _label)
  (set `self.Time` (+ _time 1))
  (if (< _time (`self.Total Game Time`))
    (bind (_gameend _team) (`self.CheckFlags`))
    (if _gameend
      (set `self.WinningTeam` _team)
      (else
        (goto _label))))
  (`self.Game Over`))

(event `self.ReceiveBeginPlay`
  (`|ExecutionSequence`
    (:`then_0`
      (`self.Counter`))
    (:`then_1`
      (`self.Multiplayer Setup`))
    (:`then_2`
      (`self.Choose Starts`))))

(event `Delete HUD`
  (for (_ _array_index) (`GameStateBase.PlayerArray` (`GameplayStatics.GetGameState`))
    (bind _asgame_hud (cast `GameHUD` (`PlayerController.GetHUD` (`GameplayStatics.GetPlayerController` _array_index))))
    (`Widget.RemoveFromParent` (`GameHUD.GetWidgetHUD` _asgame_hud))
    (`self.DisableInput` (`GameplayStatics.GetPlayerCharacter` _array_index) null)))

(event `Choose Starts`
  ;[1 1 1] Choose Starts
  (`KismetSystemLibrary.Delay` 0.7)
  (bind _outactors (`GameplayStatics.GetAllActorsOfClass` "/Game/Blueprints/Characters/BP_Character.BP_Character_C"))
  (for _array_element _outactors
    (bind _spawn (`self.Choose Start` _array_element))
    (`self.K2_SetActorLocation` _array_element (`self.K2_GetActorLocation` _spawn) false false)
    (`self.K2_SetActorRotation` (`self.K2_GetActorRotation` _spawn))))

(event `Multiplayer Setup`
  (`KismetSystemLibrary.Delay` 0.2)
  (`|ExecutionSequence`
    (:`then_0`
      (switch `/Game/Blueprints/E_NumPlayers` (`self.NumPlayers_0`)
        (:`NewEnumerator0`
          _)
        (:`NewEnumerator1`
          (`|ExecutionSequence`
            (:`then_0`
              (goto _label_2 :!via `Reset`))
            (:`then_1`
              _)))
        (:`NewEnumerator2`
          (`|ExecutionSequence`
            (:`then_0`
              (goto _label_2 :!via `Reset`))
            (:`then_1`
              (goto _label_3 :!via `Reset`))
            (:`then_2`
              _)))
        (:`NewEnumerator3`
          (`|ExecutionSequence`
            (:`then_0`
              (goto _label_2 :!via `Reset`))
            (:`then_1`
              (goto _label_3 :!via `Reset`))
            (:`then_2`
              (goto _label_4 :!via `Reset`))
            (:`then_3`
              _))))
      (bind _asbp_character (cast `/Game/Blueprints/Characters/BP_Character` (`Controller.K2_GetPawn` (`GameplayStatics.GetPlayerController` 0))))
      (set `/Game/Blueprints/Characters/BP_Character.PlayerIndexCache` 1 _asbp_character)
      (`KismetSystemLibrary.Delay` 0.2)
      (`PlayerCharacter.SetTeam` _asbp_character (`self.Team 1`))
      (set `/Game/Blueprints/Characters/BP_Character.TeamMember` 1 _asbp_character))
    (:`then_1`
      (`/Engine/EditorBlueprintResources/StandardMacros.DoOnce` true :!label _label_2
        (:`Completed`
          (bind _returnvalue (`GameplayStatics.CreatePlayer` 1))
          (bind _asbp_character_2 (cast `/Game/Blueprints/Characters/BP_Character` (`Controller.K2_GetPawn` _returnvalue)))
          (set `/Game/Blueprints/Characters/BP_Character.PlayerIndexCache` 2 _asbp_character_2)
          (switch `/Game/Blueprints/E_PVPModes` (`self.PVP Modes`)
            (:`NewEnumerator0`
              (`PlayerCharacter.SetTeam` _asbp_character_2 (`self.Team 2`))
              (set `/Game/Blueprints/Characters/BP_Character.TeamMember` 1 _asbp_character_2))
            (:`NewEnumerator1`
              (`PlayerCharacter.SetTeam` _asbp_character_2 (`self.Team 1`))
              (set `/Game/Blueprints/Characters/BP_Character.TeamMember` 2 _asbp_character_2)
              (`/Engine/EditorBlueprintResources/StandardMacros.DoOnce` false :!label _label_3
                (:`Completed`
                  (bind _returnvalue_2 (`GameplayStatics.CreatePlayer` 2))
                  (bind _asbp_character_3 (cast `/Game/Blueprints/Characters/BP_Character` (`Controller.K2_GetPawn` _returnvalue_2)))
                  (set `/Game/Blueprints/Characters/BP_Character.PlayerIndexCache` 3 _asbp_character_3)
                  (`PlayerCharacter.SetTeam` _asbp_character_3 (`self.Team 2`))
                  (set `/Game/Blueprints/Characters/BP_Character.TeamMember` 1 _asbp_character_3)
                  (`/Engine/EditorBlueprintResources/StandardMacros.DoOnce` false :!label _label_4
                    (:`Completed`
                      (bind _returnvalue_3 (`GameplayStatics.CreatePlayer` 3))
                      (bind _asbp_character_4 (cast `/Game/Blueprints/Characters/BP_Character` (`Controller.K2_GetPawn` _returnvalue_3)))
                      (set `/Game/Blueprints/Characters/BP_Character.PlayerIndexCache` 4 _asbp_character_4)
                      (`PlayerCharacter.SetTeam` _asbp_character_4 (`self.Team 2`))
                      (set `/Game/Blueprints/Characters/BP_Character.TeamMember` 2 _asbp_character_4))))))))))))

(fn `CheckFlags`
  (returns (GameEnd :type Boolean) (Team :type Integer))
  (locals (BlockTeamTest :type Integer) (NewLocalVar_0 :type "BuildArea Object Reference"))
  (bind _outactors (`GameplayStatics.GetAllActorsOfClass` "/Game/Blueprints/Construction/BP_BuildArea.BP_BuildArea_C"))
  (for _array_element _outactors
    (set `local.NewLocalVar_0` _array_element)
    (for _array_element_2 (`self.GetOverlappingActors` _array_element null)
      (bind _asflag_block (cast `FlagBlock` _array_element_2))
      (bind _m_team (`BuildArea.m_Team` _array_element))
      (if (!= _m_team (`Block.m_Team` _asflag_block))
        (return true _m_team))))
  (return false 0))

(fn `Choose Start`
  (params (Character :type "/Game/Blueprints/Characters/BP_Character Object Reference"))
  (returns (Spawn :type "/Game/Blueprints/BP_SpawnPoint Object Reference"))
  (bind _outactors (`GameplayStatics.GetAllActorsOfClass` "/Game/Blueprints/BP_SpawnPoint.BP_SpawnPoint_C"))
  (for _array_element _outactors
    (if (== (`/Game/Blueprints/BP_SpawnPoint.Team` _array_element) (`PlayerCharacter.m_Team` Character))
      (if (== (`/Game/Blueprints/BP_SpawnPoint.Player` _array_element) (`/Game/Blueprints/Characters/BP_Character.TeamMember` Character))
        (return _array_element)))))

(fn `UserConstructionScript`)