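; Marble shower game event that handles the storm's post-process and Wwise audio.
; Tick eases the post-process blend weight in and out with a sine curve at the start and end of the event's duration.
; Once the GMCapturePoints MTimer exceeds 10, a DoOnce switches music to Storm and posts thunder.
; OnEnd restores the Level_4 music state and resets that DoOnce.
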(event `self.OnEnd`
  (`AkGameplayStatics.SetState` "Music" "Level_4")
  (`KismetSystemLibrary.PrintString` "reset")
  (goto _label :!via `Reset`))

(event `self.ReceiveTick`
  (params (DeltaSeconds :type "Float (single-precision)"))
  (bind _post_blend_duration (`self.Post Blend Duration`))
  (bind _returnvalue (/ (`self.GetRunTime`) (`self.Post Blend Duration`)))
  (bind _returnvalue_2 (- (`self.GetDuration`) (`self.GetRunTime`)))
  (`|ExecutionSequence`
    (:`then_0`
      (if (< _returnvalue 1.0)
        (set `PostProcessComponent.BlendWeight` (`KismetMathLibrary.Sin` (`KismetMathLibrary.MultiplyByPi` (* _returnvalue 0.5))) (`self.PostProcess`))
        (elif (<= _returnvalue_2 _post_blend_duration)
          (set `PostProcessComponent.BlendWeight` (`KismetMathLibrary.Sin` (`KismetMathLibrary.MultiplyByPi` (* (/ _returnvalue_2 _post_blend_duration) 0.5))) (`self.PostProcess`)))))
    (:`then_1`
      (bind _asgmcapture_points (cast `GMCapturePoints` (`GameplayStatics.GetGameMode`)))
      (if (> (`BaseGameMode.m_Timer` _asgmcapture_points) 10.0)
        (`/Engine/EditorBlueprintResources/StandardMacros.DoOnce` false :!label _label
          (:`Completed`
            (`AkGameplayStatics.SetState` "Music" "Storm")
            (`AkGameplayStatics.PostEvent` "/Game/Audio/Events/Music/Thunder.Thunder")))))))

(fn `UserConstructionScript`)