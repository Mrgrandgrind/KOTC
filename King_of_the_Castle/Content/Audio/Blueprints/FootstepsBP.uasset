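; FootstepsBP is an actor Blueprint that plays surface-dependent player footstep sounds through Wwise.
; A custom event casts the owner to Pawn and runs a debug-drawn visibility trace from its location, with a zero end offset as written.
; The hit's physical surface sets the "Surface" switch (wood, light or heavy plastic, paper; wood by default).
; It then posts the Fs_player event at the impact point.
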(event `CustomEvent`
  (bind _aspawn (cast `Pawn` (`self.GetOwner`)))
  (bind _returnvalue (`self.K2_GetActorLocation` _aspawn))
  (bind _outhit (`KismetSystemLibrary.LineTraceSingle` _returnvalue (+ _returnvalue (0.0 0.0 0.0)) "TraceTypeQuery1" false (`|MakeArray` _aspawn) "ForDuration"))
  (`AkGameplayStatics.SetSwitch` "Surface" (select `EPhysicalSurface` (`GameplayStatics.GetSurfaceType` _outhit) :`SurfaceType_Default` "Wood" :`SurfaceType1` "Wood" :`SurfaceType2` "PlasticLight" :`SurfaceType3` "PlasticHeavy" :`SurfaceType4` "Paper" :!type "Name"))
  (`AkGameplayStatics.PostEventAtLocation` "/Game/Audio/Events/SFX/fs_player.fs_player" (`.ImpactPoint` (`GameplayStatics.BreakHitResult` _outhit))))

(fn `UserConstructionScript`)