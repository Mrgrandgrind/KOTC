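; BP_Marble is a physics-driven destructible marble for the marble event that deals area damage when it shatters.
; Each tick it overwrites horizontal velocity with its Direction scaled by vertical velocity, tying sideways motion to fall speed.
; On fracture it applies radial falloff environmental damage, plays force feedback and camera shake at the hit point, then makes the destructible mesh ignore Pawn collision.
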(event `self.ReceiveBeginPlay`
  (add `DestructibleComponent.OnComponentFracture` (`self.M_Marble_DM`) (delegate `OnFracture`)))

(event `OnFracture`
  (params (HitPoint :type "Vector Structure (by ref)") (HitDirection :type "Vector Structure (by ref)"))
  (`GameplayStatics.ApplyRadialDamageWithFalloff` :`BaseDamage` 120.0 :`MinimumDamage` 0.0 :`Origin` HitPoint :`DamageInnerRadius` 10.0 :`DamageOuterRadius` 820.0 :`DamageFalloff` 2.0 :`DamageTypeClass` "/Engine/EngineDamageTypes/DmgTypeBP_Environmental.DmgTypeBP_Environmental_C" :`DamageCauser` self)
  (bind _returnvalue (`GameplayStatics.SpawnForceFeedbackAtLocation` "/Game/Misc/ForceFeedback/FFE_MarbleSmash.FFE_MarbleSmash" HitPoint (struct)))
  (`ForceFeedbackComponent.AdjustAttenuation` _returnvalue (`self.AttenuationSettings`))
  (`GameplayStatics.PlayWorldCameraShake` "/Game/Blueprints/Event/MarbleEvent/BP_CameraShake.BP_CameraShake_C" HitPoint 0.0 2000.0 1.0 true)
  (`PrimitiveComponent.SetCollisionResponseToChannel` (`self.M_Marble_DM`) "ECC_Pawn" "ECR_Ignore"))

(event `self.ReceiveTick`
  (params (DeltaSeconds :type "Float (single-precision)"))
  (bind _m_marble_dm (`self.M_Marble_DM`))
  (bind _returnvalue (`PrimitiveComponent.GetPhysicsLinearVelocity` _m_marble_dm "None"))
  (bind _z (.z _returnvalue))
  (`PrimitiveComponent.SetPhysicsLinearVelocity` _m_marble_dm (`KismetMathLibrary.MakeVector` (.x (* (`self.Direction`) _z)) (.y (* (`self.Direction`) _z)) _z) false "None"))

(fn `UserConstructionScript`)