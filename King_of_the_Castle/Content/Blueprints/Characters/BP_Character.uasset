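; Character Blueprint that handles HUD setup and timed melee and special attack input.
; One second after BeginPlay it creates BP_HUD for its player controller, links itself to it, and derives charge and dodge distances from mesh bounds.
; Each attack input closes its own Gate, raises a state flag, fires the attack mid-delay, clears the flag, then reopens after a cooldown.
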(event `self.ReceiveBeginPlay`
  (bind _x (.x (`.BoxExtent` (`KismetSystemLibrary.GetComponentBounds` (`self.Mesh`)))))
  (`KismetSystemLibrary.Delay` 1.0)
  (bind _asplayer_controller (cast `PlayerController` (`self.GetController` self)))
  (bind _returnvalue (`|CreateWidget` "/Game/Blueprints/BP_HUD.BP_HUD_C" _asplayer_controller))
  (bind _output_get (set `self.HUD` _returnvalue))
  (set `/Game/Blueprints/BP_HUD.PlayerCharacter` self _output_get)
  (`UserWidget.AddToPlayerScreen` _output_get 0)
  (set `self.m_ChargeDist` _x)
  (set `self.m_DodgeDist` (* _x 3.0)))

(event `InputAction|Attack` :consume false :overrideparent false
  (params (Key :type "Key Structure" :default "AnyKey"))
  (:`Pressed`
    (`/Engine/EditorBlueprintResources/StandardMacros.Gate` false :!label _label
      (:`Exit`
        (`|ExecutionSequence`
          (:`then_0`
            (goto _label :!via `Close`))
          (:`then_1`
            (set `self.Attack` true)
            (`KismetSystemLibrary.Delay` 0.4)
            (`self.MeleeAttack`)
            (`KismetSystemLibrary.Delay` 0.2)
            (set `self.Attack` false)
            (`KismetSystemLibrary.Delay` (`self.AttackDelay`))
            (goto _label :!via `Open`)))))))

(event `InputAction|Special` :consume false :overrideparent false
  (params (Key :type "Key Structure" :default "AnyKey"))
  (:`Pressed`
    (`/Engine/EditorBlueprintResources/StandardMacros.Gate` false :!label _label_2
      (:`Exit`
        (`|ExecutionSequence`
          (:`then_0`
            (goto _label_2 :!via `Close`))
          (:`then_1`
            (set `self.Special` true)
            (`KismetSystemLibrary.Delay` 0.4)
            (`self.SpecialAttack`)
            (`KismetSystemLibrary.Delay` 0.4)
            (set `self.Special` false)
            (`KismetSystemLibrary.Delay` (`self.SpecialDelay`))
            (goto _label_2 :!via `Open`)))))))

(fn `UserConstructionScript`)