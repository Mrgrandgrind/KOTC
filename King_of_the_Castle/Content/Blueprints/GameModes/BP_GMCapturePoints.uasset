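; Capture-points game mode Blueprint that layers Wwise audio onto its parent's capture logic.
; The capture begin, capture end and captured overrides call the parent, then post the matching Wwise event on the capture point actor.
; Tick switches the Players_Capturing RTPC on a point between off and full, depending on whether its speed multiplier has reached a threshold.
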(event `self.OnCapturePointCaptureEnd`
  (params (point :type "CapturePoint Object Reference") (team :type "Integer (by ref)"))
  (`parent.OnCapturePointCaptureEnd` point team)
  (`AkGameplayStatics.PostEvent` "/Game/Audio/Events/SFX/base_capture_end.base_capture_end" point))

(event `self.OnCapturePointCaptureBegin`
  (params (point :type "CapturePoint Object Reference") (team :type "Integer (by ref)"))
  (`parent.OnCapturePointCaptureBegin` point team)
  (`AkGameplayStatics.PostEvent` "/Game/Audio/Events/SFX/base_capturing.base_capturing" point))

(event `self.OnCapturePointCaptured`
  (params (point :type "CapturePoint Object Reference"))
  (`parent.OnCapturePointCaptured` point)
  (`AkGameplayStatics.PostEvent` "/Game/Audio/Events/SFX/base_captured.base_captured" point))

(event `self.ReceiveTick`
  (params (DeltaSeconds :type "Float (single-precision)"))
  (if (< (`CapturePoint.GetSpeedMultiplier` (stale `self.OnCapturePointCaptureBegin` point)) 2.0)
    (`AkGameplayStatics.SetRTPCValue` "Players_Capturing" 0.0 0 (stale `self.OnCapturePointCaptured` point))
    (else
      (`AkGameplayStatics.SetRTPCValue` "Players_Capturing" 100.0 0 (stale `self.OnCapturePointCaptured` point)))))

(fn `UserConstructionScript`)