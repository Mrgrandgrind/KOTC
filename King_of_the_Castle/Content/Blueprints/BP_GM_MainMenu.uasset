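; BP_GM_MainMenu, a game mode by its name, holds team spawn selection and a flag-capture end check.
; ChooseStart returns the BP_SpawnPoint whose team and player slot match the given character's team and member number.
; CheckFlags scans actors overlapping each BP_BuildArea and reports game end, with that area's team, upon finding another team's FlagBlock.
; Both functions search the level with GetAllActorsOfClass on each call.
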(fn `CheckFlags`
  (returns (GameEnd :type Boolean) (Team :type Integer))
  (locals (BlockTeamTest :type Integer) (NewLocalVar_0 :type "BuildArea Object Reference"))
  (bind _outactors (`GameplayStatics.GetAllActorsOfClass` "/Game/Blueprints/Construction/BP_BuildArea.BP_BuildArea_C"))
  (for _array_element _outactors
    (set `local.NewLocalVar_0` _array_element)
    (for _array_element_2 (`self.GetOverlappingActors` _array_element null)
      (bind _asflag_block (cast `FlagBlock` _array_element_2))
      (bind _m_team (`BuildArea.m_Team` _array_element))
      (if (!= _m_team (`Block.m_Team` _asflag_block))
        (return true _m_team))))
  (return false 0))

(fn `Choose Start`
  (params (Character :type "/Game/Blueprints/Characters/BP_Character Object Reference"))
  (returns (Spawn :type "/Game/Blueprints/BP_SpawnPoint Object Reference"))
  (bind _outactors (`GameplayStatics.GetAllActorsOfClass` "/Game/Blueprints/BP_SpawnPoint.BP_SpawnPoint_C"))
  (for _array_element _outactors
    (if (== (`/Game/Blueprints/BP_SpawnPoint.Team` _array_element) (`PlayerCharacter.m_Team` Character))
      (if (== (`/Game/Blueprints/BP_SpawnPoint.Player` _array_element) (`/Game/Blueprints/Characters/BP_Character.TeamMember` Character))
        (return _array_element)))))

(fn `UserConstructionScript`)